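; BP_OfficeKey is a collectible office key pickup for the stealth game that floats and spins in place.
; The FloatingSpin timeline, started on BeginPlay, lerps the Cube's relative height and yaw.
; When BP_ThirdPersonCharacterCustom overlaps BoxCollision, the key sets that character's OfficeKeyCount to a constant 1 rather than incrementing it, then destroys itself.
; Debug strings report spawning, pickup and failed casts.
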(event OnComponentBeginOverlap(BoxCollision)
  (params (OverlappedComponent :type Primitive%20Component%20Object%20Reference) (OtherActor :type Actor%20Object%20Reference) (OtherComp :type Primitive%20Component%20Object%20Reference) (OtherBodyIndex :type Integer) (bFromSweep :type Boolean) (SweepResult :type Hit%20Result%20Structure%20%28by%20ref%29))
  (bind _asbp_third_person_character_custom (Utilities|Casting|CastToBP_ThirdPersonCharacterCustom OtherActor)
    (:then
      (Development|PrintString "Key has been Overlapped by Player" true true "(R=0.000000,G=0.660000,B=1.000000,A=1.000000)" 5.0)
      (Variables|/Game/StealthGame/Core/Characters/PlayerCharacter/BP_ThirdPersonCharacterCustom.BP_ThirdPersonCharacterCustom_C|SetOffice%20Key%20Count _asbp_third_person_character_custom (+ 0 1))
      (Development|PrintString (Utilities|String|Append "The Player has " (Utilities|String|ToString(Integer) (Variables|/Game/StealthGame/Core/Characters/PlayerCharacter/BP_ThirdPersonCharacterCustom.BP_ThirdPersonCharacterCustom_C|GetOffice%20Key%20Count _asbp_third_person_character_custom)) "office key(s)."))
      (Actor|DestroyActor) ; Destroy this key
    )
    (:CastFailed
      (Development|PrintString "Key Player Cast Failed" true true "(R=0.875000,G=0.000000,B=0.029306,A=1.000000)"))))

(event EventBeginPlay
  (Development|PrintString "This Key Exists!" true true "(R=0.989389,G=0.130208,B=1.000000,A=1.000000)")
  (bind (_direction _spin _floating) (Timeline|FloatingSpin Play)
    (:Update
      (Transformation|SetRelativeLocationAndRotation (Variables|Default|GetCube) (Math|Vector|Lerp(Vector) "0, 0, 0" "0.000000,0.000000,20.000000" _floating) (Math|Rotator|Lerp(Rotator) "0, 0, 0" "0.000000,360.000000,0.000000" _spin) false false))))

(fn ConstructionScript)