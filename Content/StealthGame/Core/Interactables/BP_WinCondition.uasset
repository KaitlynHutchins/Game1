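; BP_WinCondition is a trigger volume that ends the stealth game in a win when the custom third-person character enters its box.
; Winning requires holding the book with health above zero, or, without the book, at least 10000 gold, with no health check.
; It shows the character's win widget, clears input mappings, fades to black, then deletes the save slot and restarts the level.
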(event OnComponentBeginOverlap(Box)
  (params (OverlappedComponent :type Primitive%20Component%20Object%20Reference) (OtherActor :type Actor%20Object%20Reference) (OtherComp :type Primitive%20Component%20Object%20Reference) (OtherBodyIndex :type Integer) (bFromSweep :type Boolean) (SweepResult :type Hit%20Result%20Structure%20%28by%20ref%29))
  (bind _asbp_third_person_character_custom (Utilities|Casting|CastToBP_ThirdPersonCharacterCustom OtherActor))
  (if (Variables|/Game/StealthGame/Core/Characters/PlayerCharacter/BP_ThirdPersonCharacterCustom.BP_ThirdPersonCharacterCustom_C|GetbHasBook _asbp_third_person_character_custom)
    (if (> (Variables|/Game/StealthGame/Core/Characters/PlayerCharacter/BP_ThirdPersonCharacterCustom.BP_ThirdPersonCharacterCustom_C|GetPlayerHealth _asbp_third_person_character_custom) 0.0)
      (UserInterface|Viewport|AddtoViewport (Variables|/Game/StealthGame/Core/Characters/PlayerCharacter/BP_ThirdPersonCharacterCustom.BP_ThirdPersonCharacterCustom_C|GetYouWinWidget _asbp_third_person_character_custom) 0 :!label _label)
      (Class|EnhancedInputSubsystemInterface|ClearAllMappings (PlayerController|LocalPlayerSubsystems|GetEnhancedInputLocalPlayerSubsystem (Game|GetPlayerController 0)))
      (CameraFades|StartCameraFade :self (Game|GetPlayerCameraManager 0) :ToAlpha 1.0 :Duration 5.0) ; Fade to black (5s)
      (Utilities|FlowControl|Delay 5.0)
      (bind _asbp_third_person_character_custom_2 (Utilities|Casting|CastToBP_ThirdPersonCharacterCustom OtherActor))
      (SaveGame|DeleteGameinSlot (Variables|/Game/StealthGame/Core/Characters/PlayerCharacter/BP_ThirdPersonCharacterCustom.BP_ThirdPersonCharacterCustom_C|GetSaveGameSlot _asbp_third_person_character_custom_2)) ; Delete the save file...
      (Development|ExecuteConsoleCommand "RestartLevel" 0) ; ...then restart the level.
    )
    (elif (>= (Variables|/Game/StealthGame/Core/Characters/PlayerCharacter/BP_ThirdPersonCharacterCustom.BP_ThirdPersonCharacterCustom_C|GetGoldCount _asbp_third_person_character_custom) 10000)
      (goto _label))))

(event EventBeginPlay)

(event Collision|EventActorBeginOverlap
  (params (OtherActor :type Actor%20Object%20Reference)))

(event EventTick
  (params (DeltaSeconds :type Float%20%28single-precision%29)))

(fn ConstructionScript)